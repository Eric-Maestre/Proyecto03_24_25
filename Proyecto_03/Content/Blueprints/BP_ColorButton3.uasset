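; Third color button in a color-matching puzzle, cycling its mesh between red, green and blue when the player interacts while overlapping its collision.
; BeginB3 picks a random starting color, rerolling until it differs from the target color state held by the referenced ColorTargetVarB3.
; Each color change sets the ButtonColor material parameter, then has that target actor run CheckButtonsB3 and CheckAllBooleans to evaluate the puzzle.
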(event OnComponentBeginOverlap(Button3Collision)
  (params (OverlappedComponent :type Primitive%20Component%20Object%20Reference) (OtherActor :type Actor%20Object%20Reference) (OtherComp :type Primitive%20Component%20Object%20Reference) (OtherBodyIndex :type Integer) (bFromSweep :type Boolean) (SweepResult :type Hit%20Result%20Structure%20%28by%20ref%29))
  (Variables|Default|SetOverlapingB3 true))

(event OnComponentEndOverlap(Button3Collision)
  (params (OverlappedComponent :type Primitive%20Component%20Object%20Reference) (OtherActor :type Actor%20Object%20Reference) (OtherComp :type Primitive%20Component%20Object%20Reference) (OtherBodyIndex :type Integer))
  (Variables|Default|SetOverlapingB3 false))

(event Custom|ChangeColor
  (bind _button3mesh (Variables|Default|GetButton3Mesh))
  (bind _colortargetvarb3 (Variables|Default|GetColorTargetVarB3))
  (switch int (Variables|Default|GetColorStateB3)
    (:0
      (Rendering|Material|SetVectorParameterValueonMaterials _button3mesh "ButtonColor" "1.000000,0.000000,0.000000"))
    (:1
      (Rendering|Material|SetVectorParameterValueonMaterials _button3mesh "ButtonColor" "0.000000,1.000000,0.000000"))
    (:2
      (Rendering|Material|SetVectorParameterValueonMaterials _button3mesh "ButtonColor" "0.000000,0.000000,1.000000")))
  (Default|CheckButtonsB3 _colortargetvarb3)
  (Default|CheckAllBooleans _colortargetvarb3))

(event Custom|BeginB3
  (bind _colortargetvarb3 (Variables|Default|GetColorTargetVarB3))
  (bind _output_get (Variables|Default|SetColorStateB3 (Math|Random|RandomIntegerinRange 0 2)))
  (Math|Integer|CompareInt _output_get (Variables|/Game/Blueprints/BP_ColorTarget.BP_ColorTarget_C|GetTargetColorState (Variables|Default|GetColorTargetVarB3)) :!label _label
    (:>
      _)
    (:==
      (Variables|Default|SetColorStateB3 (Math|Random|RandomIntegerinRange 0 2))
      (goto _label))
    (:<
      _))
  (CallFunction|ChangeColor)
  (Default|CheckButtonsB3 _colortargetvarb3)
  (Default|CheckAllBooleans _colortargetvarb3))

(event EventInteract
  (params (Player :type Character%20Event%20Structure))
  (if (Variables|Default|GetOverlapingB3)
    (Variables|Default|SetColorStateB3 (Math|Integer|%(Integer) (+ (Variables|Default|GetColorStateB3) 1) 3))
    (CallFunction|ChangeColor)))

(fn ConstructionScript)