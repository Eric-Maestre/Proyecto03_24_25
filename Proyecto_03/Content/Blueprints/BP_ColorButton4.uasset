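; BP_ColorButton4 is a puzzle-style button that cycles its mesh color through red, green and blue.
; It starts on a random color, and pressing the 6 key advances it while something overlaps its Box trigger.
; ChangeColor sets the ButtonColor material parameter from the integer state, then calls CheckButtonsB4 and CheckAllBooleans on the referenced color target to re-evaluate the combination.
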(event OnComponentBeginOverlap(Box)
  (params (OverlappedComponent :type Primitive%20Component%20Object%20Reference) (OtherActor :type Actor%20Object%20Reference) (OtherComp :type Primitive%20Component%20Object%20Reference) (OtherBodyIndex :type Integer) (bFromSweep :type Boolean) (SweepResult :type Hit%20Result%20Structure%20%28by%20ref%29))
  (Variables|Default|SetOverlaping4 true))

(event OnComponentEndOverlap(Box)
  (params (OverlappedComponent :type Primitive%20Component%20Object%20Reference) (OtherActor :type Actor%20Object%20Reference) (OtherComp :type Primitive%20Component%20Object%20Reference) (OtherBodyIndex :type Integer))
  (Variables|Default|SetOverlaping4 false))

(event Custom|ChangeColor
  (bind _buttonmesh4 (Variables|Default|GetButtonMesh4))
  (bind _colortargetvarb4 (Variables|Default|GetColorTargetVarB4))
  (switch int (Variables|Default|GetColorStateB4)
    (:0
      (Rendering|Material|SetVectorParameterValueonMaterials _buttonmesh4 "ButtonColor" "1.000000,0.000000,0.000000"))
    (:1
      (Rendering|Material|SetVectorParameterValueonMaterials _buttonmesh4 "ButtonColor" "0.000000,1.000000,0.000000"))
    (:2
      (Rendering|Material|SetVectorParameterValueonMaterials _buttonmesh4 "ButtonColor" "0.000000,0.000000,1.000000")))
  (Default|CheckButtonsB4 _colortargetvarb4)
  (Default|CheckAllBooleans _colortargetvarb4))

(event EventBeginPlay
  (bind _colortargetvarb4 (Variables|Default|GetColorTargetVarB4))
  (Variables|Default|SetColorStateB4 (Math|Random|RandomIntegerinRange 0 2))
  (CallFunction|ChangeColor)
  (Default|CheckButtonsB4 _colortargetvarb4)
  (Default|CheckAllBooleans _colortargetvarb4))

(event Input|KeyboardEvents|6
  (params (Key :type Key%20Structure :default "None"))
  (:Pressed
    (if (Variables|Default|GetOverlaping4)
      (Variables|Default|SetColorStateB4 (Math|Integer|%(Integer) (+ (Variables|Default|GetColorStateB4) 1) 3))
      (CallFunction|ChangeColor))))

(fn ConstructionScript)