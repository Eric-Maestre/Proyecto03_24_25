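; BP_ColorTarget is the target of a color-matching puzzle that removes a door when four buttons match its color.
; On BeginPlay it picks red, green or blue at random and sets its mesh's material color parameter.
; Each button has a check event that latches a flag when its color state matches; the flags are never cleared here.
; Once all four flags are true, CheckAllBooleans destroys the referenced door.
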(event Custom|CheckButtons
  (Math|Integer|CompareInt (Variables|Default|GetTargetColorState) (Variables|/Game/Blueprints/BP_ColorButton.BP_ColorButton_C|GetColorState (Variables|Default|GetColorButtonVar))
    (:==
      (if true
        (Variables|Default|SetButton1Check true)
        (CallFunction|CheckAllBooleans)))))

(event Custom|ChangeColor
  (bind _colortargetmesh (Variables|Default|GetColorTargetMesh))
  (switch int (Variables|Default|GetTargetColorState)
    (:0
      (Rendering|Material|SetVectorParameterValueonMaterials _colortargetmesh "ButtonColor" "1.000000,0.000000,0.000000"))
    (:1
      (Rendering|Material|SetVectorParameterValueonMaterials _colortargetmesh "ButtonColor" "0.000000,1.000000,0.000000"))
    (:2
      (Rendering|Material|SetVectorParameterValueonMaterials _colortargetmesh "ButtonColor" "0.000000,0.000000,1.000000")))
  (CallFunction|CheckAllBooleans))

(event Custom|CheckButtonsB2
  (Math|Integer|CompareInt (Variables|Default|GetTargetColorState) (Variables|/Game/Blueprints/BP_ColorButton2.BP_ColorButton2_C|GetColorStateB2 (Variables|Default|GetColorButton2Var))
    (:==
      (if true
        (Variables|Default|SetButton2Check true)
        (CallFunction|CheckAllBooleans)))))

(event Custom|CheckAllBooleans
  (if (Math|Boolean|ANDBoolean (Variables|Default|GetButton1Check) (Variables|Default|GetButton2Check) (Variables|Default|GetButton3Check) (Variables|Default|GetButton4Check))
    (Actor|DestroyActor (Variables|Default|GetDoorVar))))

(event Custom|CheckButtonsB3
  (Math|Integer|CompareInt (Variables|Default|GetTargetColorState) (Variables|/Game/Blueprints/BP_ColorButton3.BP_ColorButton3_C|GetColorStateB3 (Variables|Default|GetColorButton3Var))
    (:==
      (if true
        (Variables|Default|SetButton3Check true)
        (CallFunction|CheckAllBooleans)))))

(event Custom|CheckButtonsB4
  (Math|Integer|CompareInt (Variables|Default|GetTargetColorState) (Variables|/Game/Blueprints/BP_ColorButton4.BP_ColorButton4_C|GetColorStateB4 (Variables|Default|GetColorButton4Var))
    (:==
      (if true
        (Variables|Default|SetButton4Check true)
        (CallFunction|CheckAllBooleans)))))

(event EventBeginPlay
  (Variables|Default|SetTargetColorState (Math|Random|RandomIntegerinRange 0 2))
  (CallFunction|ChangeColor))

(fn ConstructionScript)