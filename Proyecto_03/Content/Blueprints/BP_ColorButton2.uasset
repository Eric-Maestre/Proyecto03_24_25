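; Color puzzle button actor that cycles its mesh between red, green and blue.
; It starts on a random color, and pressing the 8 key while something overlaps its collision advances to the next one.
; Each change sets the ButtonColor material parameter and calls CheckButtonsB2 on a referenced target, which is also called on BeginPlay.
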(event OnComponentBeginOverlap(Button2Collision)
  (params (OverlappedComponent :type Primitive%20Component%20Object%20Reference) (OtherActor :type Actor%20Object%20Reference) (OtherComp :type Primitive%20Component%20Object%20Reference) (OtherBodyIndex :type Integer) (bFromSweep :type Boolean) (SweepResult :type Hit%20Result%20Structure%20%28by%20ref%29))
  (Variables|Default|SetOverlapingB2 true))

(event OnComponentEndOverlap(Button2Collision)
  (params (OverlappedComponent :type Primitive%20Component%20Object%20Reference) (OtherActor :type Actor%20Object%20Reference) (OtherComp :type Primitive%20Component%20Object%20Reference) (OtherBodyIndex :type Integer))
  (Variables|Default|SetOverlapingB2 false))

(event Custom|ChangeColor
  (bind _button2mesh (Variables|Default|GetButton2Mesh))
  (switch int (Variables|Default|GetColorStateB2)
    (:0
      (Rendering|Material|SetVectorParameterValueonMaterials _button2mesh "ButtonColor" "1.000000,0.000000,0.000000"))
    (:1
      (Rendering|Material|SetVectorParameterValueonMaterials _button2mesh "ButtonColor" "0.000000,1.000000,0.000000"))
    (:2
      (Rendering|Material|SetVectorParameterValueonMaterials _button2mesh "ButtonColor" "0.000000,0.000000,1.000000")))
  (Default|CheckButtonsB2 (Variables|Default|GetColorTargetVarB2)))

(event EventBeginPlay
  (Variables|Default|SetColorStateB2 (Math|Random|RandomIntegerinRange 0 2))
  (CallFunction|ChangeColor)
  (Default|CheckButtonsB2 (Variables|Default|GetColorTargetVarB2)))

(event Input|KeyboardEvents|8
  (params (Key :type Key%20Structure :default "None"))
  (:Pressed
    (if (Variables|Default|GetOverlapingB2)
      (Variables|Default|SetColorStateB2 (Math|Integer|%(Integer) (+ (Variables|Default|GetColorStateB2) 1) 3))
      (CallFunction|ChangeColor))))

(fn ConstructionScript)